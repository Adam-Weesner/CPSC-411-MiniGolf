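; Game mode for a golf game that runs the startup flow, level start, scoring medals and music.
; BeginPlay lowers scalability via console commands, streams in level0 behind a timed splash screen, then shows the main menu with a looping sequence, a stationary ball and music.
; FinishLoading swaps to the level UI, resets points and enables ball physics.
; DetermineMedal rates points against per-level thresholds with crowd sounds, and ToggleMusic fades music volume.
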(event `self.ReceiveBeginPlay`
  (bind _returnvalue (`GameplayStatics.GetPlayerController` 0))
  (bind _grasslands (`self.Grasslands`))
  (`self.SetScalability`)
  (bind _returnvalue_2 (`|CreateWidget` "/Game/UI/SplashScreen.SplashScreen_C"))
  (`UserWidget.AddToViewport` _returnvalue_2 0)
  (`GameplayStatics.LoadStreamLevel` "level0" true)
  (`KismetSystemLibrary.Delay` 1.5)
  (`Widget.RemoveFromParent` _returnvalue_2)
  (bind _returnvalue_3 (`|CreateWidget` "/Game/UI/MainMenu.MainMenu_C" _returnvalue))
  (`UserWidget.AddToViewport` _returnvalue_3 0)
  (set `PlayerController.bShowMouseCursor` true _returnvalue)
  (`WidgetBlueprintLibrary.SetInputMode_UIOnlyEx` _returnvalue _returnvalue_3)
  (bind (_outactor _returnvalue_4) (`LevelSequencePlayer.CreateLevelSequencePlayer` "/Game/Cinematics/FadeIn.FadeIn"))
  (`MovieSceneSequencePlayer.Play` _returnvalue_4)
  (bind (_outactor_2 _returnvalue_5) (`LevelSequencePlayer.CreateLevelSequencePlayer` "/Game/Cinematics/MainMenu.MainMenu"))
  (bind _output_get (set `self.MenuPlayer` _returnvalue_5))
  (`MovieSceneSequencePlayer.PlayLooping` _output_get -1)
  (`KismetSystemLibrary.Delay` 2.0)
  (bind _asgolf_ball (cast `/Game/Characters/GolfBall` (`GameplayStatics.GetPlayerPawn` 0)))
  (`/Game/Characters/GolfBall.SetStationary` _asgolf_ball true)
  (bind _asbp_game_instance (cast `/Game/Blueprints/BP_GameInstance` (`GameplayStatics.GetGameInstance`)))
  (switch `int` (`/Game/Blueprints/BP_GameInstance.CurrentGroup` _asbp_game_instance)
    (:`0`
      (`AudioComponent.Play` _grasslands 0.0))
    (:`1`
      (`AudioComponent.Play` _grasslands 0.0))))

(fn `DetermineMedal`
  (bind _points (`self.Points`))
  (bind _levelindex (`self.LevelIndex`))
  (bind _output (`|GetArrayItem` (`self.GoldValue`) _levelindex))
  (if (< _points 0)
    (set `self.Medal` 0)
    (`GameplayStatics.PlaySound2D` "/Game/Audio/Sounds/Crowd/Crowd_Disappointed.Crowd_Disappointed" 1.0 1.0 0.0 null null)
    (elif (`KismetMathLibrary.InRange_IntInt` _points (`|GetArrayItem` (`self.SilverValue`) _levelindex) _output)
      (set `self.Medal` 1)
      (`GameplayStatics.PlaySound2D` "/Game/Audio/Sounds/Crowd/Crowd_Clapping.Crowd_Clapping" 1.0 1.0 0.0 null null)
      (elif (>= _points _output)
        (set `self.Medal` 2)
        (`GameplayStatics.PlaySound2D` "/Game/Audio/Sounds/Crowd/Crowd_Cheering.Crowd_Cheering" 1.0 1.0 0.0 null null)))))

(fn `FinishLoading`
  (`WidgetLayoutLibrary.RemoveAllWidgets`)
  (bind (_outactor _returnvalue) (`LevelSequencePlayer.CreateLevelSequencePlayer` "/Game/Cinematics/FadeIn.FadeIn"))
  (`MovieSceneSequencePlayer.Play` _returnvalue)
  (`WidgetBlueprintLibrary.SetInputMode_GameAndUIEx` (`GameplayStatics.GetPlayerController` 0) null "DoNotLock" false)
  (bind _returnvalue_2 (`|CreateWidget` "/Game/UI/UI_Level.UI_Level_C"))
  (bind _output_get (set `self.UILevelVar` _returnvalue_2))
  (`UserWidget.AddToViewport` _output_get 0)
  (bind _asbp_game_mode (cast `/Game/Blueprints/BP_GameMode` (`GameplayStatics.GetGameMode`)))
  (set `/Game/Blueprints/BP_GameMode.Points` 0 _asbp_game_mode)
  (`MovieSceneSequencePlayer.Stop` (`/Game/Blueprints/BP_GameMode.MenuPlayer` _asbp_game_mode))
  (`GameplayStatics.PlaySound2D` "/Game/Audio/Sounds/UI/UI_Level_Select.UI_Level_Select" 1.0 1.0 0.0 null null)
  (bind _asgolf_ball (cast `/Game/Characters/GolfBall` (`GameplayStatics.GetPlayerPawn` 0)))
  (`PrimitiveComponent.SetSimulatePhysics` (`/Game/Characters/GolfBall.GolfBall` _asgolf_ball) true))

(fn `SetScalability`
  (`KismetSystemLibrary.ExecuteConsoleCommand` "sg.ResolutionQuality 69" null)
  (`KismetSystemLibrary.ExecuteConsoleCommand` "sg.ViewDistanceQuality 0" null)
  (`KismetSystemLibrary.ExecuteConsoleCommand` "sg.AntiAliasingQuality 0" null)
  (`KismetSystemLibrary.ExecuteConsoleCommand` "sg.PostProcessQuality 0" null)
  (`KismetSystemLibrary.ExecuteConsoleCommand` "sg.ShadowQuality 0" null)
  (`KismetSystemLibrary.ExecuteConsoleCommand` "sg.TextureQuality 0" null)
  (`KismetSystemLibrary.ExecuteConsoleCommand` "sg.EffectsQuality 0" null))

(fn `ToggleMusic`
  (bind _grasslands (`self.Grasslands`))
  (`GameplayStatics.PlaySound2D` "/Game/Audio/Sounds/UI/UI_Button.UI_Button" 1.0 1.0 0.0 null null)
  (if (`self.IsMusicOn`)
    (`AudioComponent.AdjustVolume` _grasslands 1.0 0.001)
    (set `self.IsMusicOn` false)
    (else
      (`AudioComponent.AdjustVolume` _grasslands 1.0 1.0)
      (set `self.IsMusicOn` true))))

(fn `UserConstructionScript`)